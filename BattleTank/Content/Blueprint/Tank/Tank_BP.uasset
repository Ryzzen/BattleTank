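; Player-controlled tank Blueprint that wires up the tank's components and routes input for driving, aiming and firing.
; BeginPlay passes barrel and turret to the turret system, initialises TankMovement with both tracks, and adds the player UI to the viewport.
; Move axes feed TankMovement intents for throttle and turning, while Fire calls a function defined outside these graphs.
; A separate InputSetup graph rotates the azimuth gimbal and spring arm to aim, scaled by delta time.
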(event `self.ReceiveBeginPlay`
  (`self.SetTurretSystemReference` (`self.TankBarrel`) (`self.Turret`))
  (`TankMovementComponent.Initialise` (`self.TankMovement`) (`self.LeftTrack`) (`self.RightTrack`))
  (bind _returnvalue (`|CreateWidget` "/Game/UI/PlayerUI.PlayerUI_C"))
  (`UserWidget.AddToViewport` _returnvalue 0))

(event `InputAction|Fire`
  (params (Key :type "Key Structure"))
  (:`Pressed`
    (`self.Fire`)))

(event `InputAxis|Move Forward`
  (params (AxisValue :type "Float (single-precision)"))
  (`TankMovementComponent.IntendMoveForward` (`self.TankMovement`) AxisValue))

(event `InputAxis|Move Backward`
  (params (AxisValue :type "Float (single-precision)"))
  (`TankMovementComponent.IntendMoveForward` (`self.TankMovement`) AxisValue))

(event `InputAxis|Move Left`
  (params (AxisValue :type "Float (single-precision)"))
  (`TankMovementComponent.IntendTurnRight` (`self.TankMovement`) AxisValue))

(event `InputAxis|Move Right`
  (params (AxisValue :type "Float (single-precision)"))
  (`TankMovementComponent.IntendTurnRight` (`self.TankMovement`) AxisValue))

(event `InputAxis|AimAzimuth`
  (params (AxisValue :type "Float (single-precision)"))
  (`SceneComponent.K2_AddLocalRotation` (`self.AzimuthGimble`) (`KismetMathLibrary.MakeRotator` 0.0 0.0 (* AxisValue (`GameplayStatics.GetWorldDeltaSeconds`) 100.0)) false false))

(event `InputAxis|AimElevation`
  (params (AxisValue :type "Float (single-precision)"))
  (`SceneComponent.K2_AddLocalRotation` (`self.SpringArm`) (`KismetMathLibrary.MakeRotator` 0.0 (* (`GameplayStatics.GetWorldDeltaSeconds`) AxisValue 100.0)) false false))

(fn `UserConstructionScript`)